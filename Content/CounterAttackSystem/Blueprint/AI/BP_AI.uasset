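; BP_AI is the enemy AI in the counter attack system, attacking a given target and showing a counter notification widget.
; Attack stores the target and tells CounterSystemComponent to start the attack on the server.
; While active, a timeline eases the actor's yaw toward the target, replicating each rotation through a Server-to-Multicast event pair.
; A separate event toggles the counter notification widget's visibility.
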(event `Attack`
  (params (TargetAttack :type "Actor Object Reference"))
  ;[0 0.05001 0.09896] Attack To Player
  (set `self.TargetAttack` TargetAttack)
  (`/Game/CounterAttackSystem/Blueprint/Component/CAS_Component.Server_StartAttack` (`self.CounterSystemComponent`)))

(event `StartRotateToPlayer`
  (bind _targetattack (`self.TargetAttack`))
  (bind (_returnvalue_roll _returnvalue_pitch _returnvalue_yaw) (`KismetMathLibrary.BreakRotator` (`KismetMathLibrary.FindLookAtRotation` (`self.K2_GetActorLocation`) (`self.K2_GetActorLocation` _targetattack))))
  ;[0 0.05001 0.09896] Rotate To Player
  (`Timeline|Rotation` :!via `PlayFromStart` :!label _label
    (:`Update`
      (`/Engine/EditorBlueprintResources/StandardMacros.IsValid` _targetattack
        (:`Is Valid`
          (`self.Server_RotateTo` (`KismetMathLibrary.RInterpTo` (`self.K2_GetActorRotation`) (`KismetMathLibrary.MakeRotator` 0.0 0.0 _returnvalue_yaw) (`GameplayStatics.GetWorldDeltaSeconds`) 20.0)))))))

(event `StopRotateToPlayer`
  ;[0 0.05001 0.09896] Rotate To Player
  (goto _label :!via `Stop`))

(event `Server_RotateTo`
  (params (Rotation :type "Rotator Structure"))
  ;[0 0.05001 0.09896] Rotate To Player
  (`self.Multicast_RotateTo` Rotation))

(event `Multicast_RotateTo`
  (params (Rotation :type "Rotator Structure"))
  ;[0 0.05001 0.09896] Rotate To Player
  (`self.K2_SetActorRotation` Rotation))

(event `ShowCounterNotifWidget`
  (params (Value :type Boolean))
  ;[0 0.05001 0.09896] Show or Hide Counter Notif Widget
  (`SceneComponent.SetHiddenInGame` (`self.CounterNotifWdiget`) (not Value) false))

(fn `UserConstructionScript`)