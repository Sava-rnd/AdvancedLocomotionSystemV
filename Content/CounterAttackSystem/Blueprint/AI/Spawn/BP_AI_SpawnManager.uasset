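; Spawn manager that keeps a single BP_AI enemy in the level, spawning a replacement when it dies.
; It picks a random BP_AI_SpawnLocation, excluding the previous one unless only one exists, and spawns the AI there with BT_AI.
; A looping timer polls the AI's CAS_Component for owner death, then respawns after a short delay.
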(event `self.ReceiveBeginPlay`
  (`self.Find and Spawn AI`))

(event `Find and Spawn AI`
  (`KismetArrayLibrary.Array_Clear` (`self.AI_Spawner`))
  (bind _outactors (`GameplayStatics.GetAllActorsOfClass` "/Game/CounterAttackSystem/Blueprint/AI/Spawn/BP_AI_SpawnLocation.BP_AI_SpawnLocation_C"))
  (set `self.AI_SpawnerFoundLength` (`KismetArrayLibrary.Array_Length` _outactors))
  (for _array_element _outactors
    (if (!= _array_element (`self.LastSpawner`))
      (`KismetArrayLibrary.Array_AddUnique` (`self.AI_Spawner`) _array_element :!label _label)
      (elif (== (`self.AI_SpawnerFoundLength`) 1)
        (goto _label))))
  (`KismetSystemLibrary.K2_ClearAndInvalidateTimerHandle` (`self.Timer`))
  (bind _output_get (set `self.LastSpawner` (`KismetArrayLibrary.Array_Random` (`self.AI_Spawner`))))
  (`self.SpawnAI` (`self.GetTransform` _output_get)))

(event `SpawnAI`
  (params (Transform :type "Transform Structure"))
  (bind _returnvalue (`AIBlueprintHelperLibrary.SpawnAIFromClass` "/Game/CounterAttackSystem/Blueprint/AI/BP_AI.BP_AI_C" "/Game/CounterAttackSystem/Blueprint/AI/BT_AI.BT_AI" (.location Transform) (.rotation Transform) true null))
  (set `self.AI_Actor` _returnvalue)
  (bind _returnvalue_2 (`KismetSystemLibrary.K2_SetTimerDelegate` (delegate `CheckToSpawnAgain`) 0.5 true))
  (set `self.Timer` _returnvalue_2))

(event `CheckToSpawnAgain`
  (bind _ai_actor (`self.AI_Actor`))
  (`/Engine/EditorBlueprintResources/StandardMacros.IsValid` _ai_actor
    (:`Is Valid`
      (if (`/Game/CounterAttackSystem/Blueprint/Component/CAS_Component.IsOwnerDead` (`self.GetComponentByClass` _ai_actor "/Game/CounterAttackSystem/Blueprint/Component/CAS_Component.CAS_Component_C"))
        (`KismetSystemLibrary.Delay` 0.65) ; The delay respawn AI
        (`self.Find and Spawn AI`)))))

(fn `UserConstructionScript`)