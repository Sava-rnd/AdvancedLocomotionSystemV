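; Camera rig actor for the Counter Attack System that creates cinematic shots of an Attacker and Victim pair.
; CinematicCameraSettings sets the spring arm's length, world rotation and offset, then spawns a CAS_CineCamera and snap-attaches it to the arm.
; A target choice of None, Attacker or Victim drives look-at tracking and the focus-tracking actor, alongside a manual focus distance.
; The function returns the configured camera to its caller.
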(fn `Cinematic Camera Settings`
  (params (Attacker :type "Character Object Reference") (Victim :type "Character Object Reference") (`Target Arm Length` :type "Float (double-precision)") (`New Rotation` :type "Rotator Structure") (`Target Offset` :type "Vector Structure") (`Draw Debug Camera Tracking` :type Boolean) (`Focus Tracking Target` :type "/Game/CounterAttackSystem/Blueprint/Enum/E_CounterActor Enum" :default "NewEnumerator4") (`Manual Focus Distance` :type "Float (single-precision)"))
  (returns (CineCamera :type "CineCameraActor Object Reference"))
  (locals (L_CineCamera :type "/Game/CounterAttackSystem/Blueprint/Camera/CAS_CineCamera Object Reference") (L_Attacker :type "Character Object Reference") (L_Victim :type "Character Object Reference"))
  (bind _springarm (`self.SpringArm`))
  (bind _l_cinecamera (`local.L_CineCamera`))
  (bind _returnvalue (select `/Game/CounterAttackSystem/Blueprint/Enum/E_CounterActor` `Focus Tracking Target` :`NewEnumerator0` (`|ConvertAsset` (`local.L_Attacker`)) :`NewEnumerator5` (`|ConvertAsset` (`local.L_Victim`)) :!type "Actor Soft Object Reference"))
  ;[1 1 1] Camera Setting for Rotation & Target Tracking Cine Camera
  (set `local.L_Attacker` Attacker)
  (set `local.L_Victim` Victim)
  (set `SpringArmComponent.TargetArmLength` `Target Arm Length` _springarm)
  (`SceneComponent.K2_SetWorldRotation` _springarm `New Rotation` false false)
  (set `SpringArmComponent.TargetOffset` `Target Offset` _springarm)
  (bind _returnvalue_2 (`|SpawnActorFromClass` "/Game/CounterAttackSystem/Blueprint/Camera/CAS_CineCamera.CAS_CineCamera_C" (`SceneComponent.K2_GetComponentToWorld` (`self.SpringArm`)) "AlwaysSpawn" "OverrideRootScale" null null))
  (set `local.L_CineCamera` _returnvalue_2)
  (`self.K2_AttachToComponent` (`local.L_CineCamera`) (`self.SpringArm`) "None" "SnapToTarget" "SnapToTarget" "SnapToTarget" true)
  (set `CineCameraActor.LookatTrackingSettings` (make `CameraLookatTrackingSettings` (`|EnumInequality` `Focus Tracking Target` "NewEnumerator4") `Draw Debug Camera Tracking` 0.0 _returnvalue) _l_cinecamera)
  (set `CineCameraComponent.FocusSettings` (make `CameraFocusSettings` "Manual" `Manual Focus Distance` (make `CameraTrackingFocusSettings` _returnvalue)) (`CineCameraActor.GetCineCameraComponent` _l_cinecamera))
  (return (`local.L_CineCamera`)))

(fn `UserConstructionScript`)