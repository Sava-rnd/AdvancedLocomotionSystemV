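; Anim notify for counter attack animations that fires hit feedback and, on the final hit, finishes the counter.
; If the character is locally controlled, it asks its CAS_Component to play the configured sound and camera shake through the server at the character's location.
; When flagged as final hit with a valid CounterVictim, it triggers the victim's delayed death ragdoll and calls EndCounter on the attacker, without a local-control check.
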(fn `GetNotifyName`
  (returns (ReturnValue :type String))
  (return (`self.Notify Name`)))

(fn `Received_Notify`
  (params (MeshComp :type "SkeletalMeshComponent Object Reference") (Animation :type "AnimSequenceBase Object Reference") (EventReference :type "AnimNotifyEventReference Structure (by ref)"))
  (returns (ReturnValue :type Boolean))
  (bind _ascharacter (cast `Character` (`ActorComponent.GetOwner` MeshComp)))
  (if (`Pawn.IsLocallyControlled` _ascharacter)
    (bind _returnvalue (`Actor.GetComponentByClass` _ascharacter "/Game/CounterAttackSystem/Blueprint/Component/CAS_Component.CAS_Component_C"))
    (bind _returnvalue_2 (`Actor.K2_GetActorLocation` _ascharacter))
    (`/Game/CounterAttackSystem/Blueprint/Component/CAS_Component.Server_PlaySound` _returnvalue (`self.Sound`) _returnvalue_2)
    (`/Game/CounterAttackSystem/Blueprint/Component/CAS_Component.Server_PlayCameraShake` _returnvalue (`self.CameraShake`) _returnvalue_2))
  (if (`self.IsFinalHit?`)
    (bind _countervictim (`/Game/CounterAttackSystem/Blueprint/Component/CAS_Component.CounterVictim` _returnvalue))
    (`/Engine/EditorBlueprintResources/StandardMacros.IsValid` _countervictim
      (:`Is Valid`
        (`/Game/CounterAttackSystem/Blueprint/Component/CAS_Component.DeadRagdoll` (`Actor.GetComponentByClass` _countervictim "/Game/CounterAttackSystem/Blueprint/Component/CAS_Component.CAS_Component_C") (`self.RagdollDelay`) _countervictim)
        (`/Game/CounterAttackSystem/Blueprint/Component/CAS_Component.End Counter` _returnvalue))))
  (return false))