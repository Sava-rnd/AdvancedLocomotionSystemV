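; Anim notify state that marks the window during an AI attack montage or animation when its target can counter.
; On begin, it casts the owner to BP_AI and opens a counter of the configured CounterType on the CAS_Component of the AI's TargetAttack, passing the AI as initiator.
; On end, it closes that window with a fixed counter type.
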(fn `Received_NotifyBegin`
  (params (MeshComp :type "SkeletalMeshComponent Object Reference") (Animation :type "AnimSequenceBase Object Reference") (TotalDuration :type "Float (single-precision)") (EventReference :type "AnimNotifyEventReference Structure (by ref)"))
  (returns (ReturnValue :type Boolean))
  (bind _asbp_ai (cast `/Game/CounterAttackSystem/Blueprint/AI/BP_AI` (`ActorComponent.GetOwner` MeshComp)))
  (bind _targetattack (`/Game/CounterAttackSystem/Blueprint/AI/BP_AI.TargetAttack` _asbp_ai))
  (`/Engine/EditorBlueprintResources/StandardMacros.IsValid` _targetattack
    (:`Is Valid`
      (`/Game/CounterAttackSystem/Blueprint/Component/CAS_Component.OpenClose_Counter` (`Actor.GetComponentByClass` _targetattack "/Game/CounterAttackSystem/Blueprint/Component/CAS_Component.CAS_Component_C") true (`self.CounterType`) _asbp_ai)
      (return false))))

(fn `Received_NotifyEnd`
  (params (MeshComp :type "SkeletalMeshComponent Object Reference") (Animation :type "AnimSequenceBase Object Reference") (EventReference :type "AnimNotifyEventReference Structure (by ref)"))
  (returns (ReturnValue :type Boolean))
  (bind _asbp_ai (cast `/Game/CounterAttackSystem/Blueprint/AI/BP_AI` (`ActorComponent.GetOwner` MeshComp)))
  (bind _targetattack (`/Game/CounterAttackSystem/Blueprint/AI/BP_AI.TargetAttack` _asbp_ai))
  (`/Engine/EditorBlueprintResources/StandardMacros.IsValid` _targetattack
    (:`Is Valid`
      (`/Game/CounterAttackSystem/Blueprint/Component/CAS_Component.OpenClose_Counter` (`Actor.GetComponentByClass` _targetattack "/Game/CounterAttackSystem/Blueprint/Component/CAS_Component.CAS_Component_C") false "NewEnumerator4" _asbp_ai)
      (return false))))