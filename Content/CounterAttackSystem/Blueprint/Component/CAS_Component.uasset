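; Character component for a melee counter-attack system, with optional ragdoll death and a simple random AI attack.
; While the counter window is open, StartCounter targets the nearest traced AI and picks paired montages from a data table by counter type and relative direction, falling back to Front.
; It aligns the attacker, ignores pawn collision and can blend to a cinematic camera until EndCounter.
; State, montages and movement replicate through Server-to-Multicast events.
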(event `self.ReceiveBeginPlay`
  ;[0 0.05001 0.09896] Begin Play
  (bind _ascharacter (cast `Character` (`self.GetOwner`)))
  (set `self.OwnerAttacker` _ascharacter)
  ;[1 0.7639 0.1963] Create controls widget. Delete this if you dont want to use it
  (bind _asplayer_controller (cast `PlayerController` (`Pawn.GetController` (`Actor.Instigator` (`self.GetOwner`)))))
  (bind _returnvalue (`|CreateWidget` "/Game/CounterAttackSystem/Blueprint/Widget/WB_Controls.WB_Controls_C" _asplayer_controller))
  (`UserWidget.AddToViewport` _returnvalue 0))

(event `Start Counter`
  (bind _ownerattacker (`self.OwnerAttacker`))
  (bind _cinematicsettings (`self.CinematicSettings`))
  (bind ((`UseCinematicCamera?_50_520533EA4FD000095C4B4381EFEA064C` _usecinematiccamera_) (`UseCameraFadeSwitchTransition?_87_DECDAFF841D0DECFAA41569E1A7BF05B` _usecamerafadeswitchtransition_) (`HoldtimeCounter_88_9E203B6C49E9817CD70B64B810EA6FB9` _holdtimecounter)) (break `/Game/CounterAttackSystem/Blueprint/Struct/S_CinematicSettings` _cinematicsettings))
  (bind (_attackermontage _attackerdelaystart _attackerplayrate _victimmontage _victimdelaystart _victimplayrate) (break `/Game/CounterAttackSystem/Blueprint/Struct/S_CounterMontageSetting` (`self.Montage Settings`)))
  (bind _returnvalue (`Actor.K2_GetActorLocation` _ownerattacker))
  ;[0 0.05001 0.09896] Start Counter
  (if (not (`self.InCounter`))
    (`/Engine/EditorBlueprintResources/StandardMacros.IsValid` _ownerattacker
      (:`Is Valid`
        (bind (_outhits _returnvalue_2) (`KismetSystemLibrary.SphereTraceMulti` _returnvalue _returnvalue (`self.RadiusTriggerDetection`) "TraceTypeQuery1" false (`|MakeArray` _ownerattacker :!type "Actor Object Reference") (`self.Trigger Draw Debug Type`)))
        (`KismetArrayLibrary.Array_Clear` (`self.VictimTemp`))
        (for _array_element _outhits
          (if _returnvalue_2
            (bind _ascharacter (cast `Character` (`.HitActor` (`GameplayStatics.BreakHitResult` _array_element))))
            (`/Engine/EditorBlueprintResources/StandardMacros.IsValid` (`AIBlueprintHelperLibrary.GetAIController` _ascharacter)
              (:`Is Valid`
                (`KismetArrayLibrary.Array_AddUnique` (`self.VictimTemp`) _ascharacter)))))
        (bind _ascharacter_2 (cast `Character` (`.ReturnValue` (`GameplayStatics.FindNearestActor` _returnvalue (`self.VictimTemp`)))))
        (set `self.CounterVictim` _ascharacter_2)
        (if (`self.CanCounter?`)
          (bind _returnvalue_3 (`|GetDataTableRow` (`self.DT_Counter`) "Fist_Counter")
            (:`then`
              (bind (_counter_settings_direction _counterdirection _success_) (`self.Get Counter Settings` _returnvalue_3 (`self.SendingCounterType`)))
              (if _success_
                (`self.Server_InCounter` true)
                (bind (_distancecounter _montagesettings _cinematicsettings_2) (break `/Game/CounterAttackSystem/Blueprint/Struct/S_CounterSetting` _counter_settings_direction))
                (set `self.DistanceCounter` _distancecounter)
                (set `self.Montage Settings` _montagesettings)
                (set `self.CinematicSettings` _cinematicsettings_2)
                ;;[1 1 1] Spawn Cinematic Camera
                (`self.Spawn Cinematic Camera` (`self.OwnerAttacker`) (`self.CounterVictim`) _cinematicsettings true)
                (`KismetSystemLibrary.Delay` (select `bool` _usecinematiccamera_ :`true` _holdtimecounter :!type "Float (single-precision)")) ; Give time camera to switching before counter. Only if cinematic is true
                ;;[1 1 1] Play Counter Montage
                (`self.PlayAttackerMontage` (`self.OwnerAttacker`) _attackermontage _attackerplayrate _attackerdelaystart)
                (`self.PlayVictimMontage` (`self.CounterVictim`) _victimmontage _victimplayrate _victimdelaystart)
                (`self.MoveRotateAttackerToVictim` (`self.OwnerAttacker`) (`self.CounterVictim`) (`self.DistanceCounter`) (select `/Game/CounterAttackSystem/Blueprint/Enum/E_TriggerCounterDirection` _counterdirection :`NewEnumerator1` 180.0 :`NewEnumerator2` 90.0 :`NewEnumerator3` -90.0) _counterdirection)
                (else
                  (`self.End Counter`))))))))))

(event `Server_InCounter`
  (params (Value :type Boolean))
  ;[0 0.05001 0.09896] Start Counter
  (`self.Multicast_InCounter` Value))

(event `Multicast_InCounter`
  (params (Value :type Boolean))
  ;[0 0.05001 0.09896] Start Counter
  (bind _output_get (set `self.InCounter` Value))
  (if _output_get
    (`self.OnCounterStart`)
    (else
      (`self.OnCounterEnd`))))

(event `End Counter`
  ;[0 0.05001 0.09896] End Counter
  (if (`self.InCounter`)
    (`self.Server_Pawn_Collision_Response` "ECR_Block" (`self.OwnerAttacker`))
    (`self.Spawn Cinematic Camera` (`self.OwnerAttacker`) (`self.CounterVictim`) (`self.CinematicSettings`))
    (set `self.CounterData` (struct))
    (set `self.CounterVictim` null)
    (`self.Server_InCounter` false)))

(event `PlayAttackerMontage`
  (params (Character :type "Character Object Reference") (Montage :type "AnimMontage Object Reference") (PlayRate :type "Float (double-precision)") (Delay :type "Float (double-precision)"))
  ;[0 0.05001 0.09896] Animation Montage
  (`KismetSystemLibrary.Delay` Delay)
  (`self.Server_PlayMontage` Character Montage PlayRate))

(event `PlayVictimMontage`
  (params (Character :type "Character Object Reference") (Montage :type "AnimMontage Object Reference") (PlayRate :type "Float (double-precision)") (Delay :type "Float (double-precision)"))
  ;[0 0.05001 0.09896] Animation Montage
  (`KismetSystemLibrary.Delay` Delay)
  (`self.Server_PlayMontage` Character Montage PlayRate))

(event `Spawn Cinematic Camera`
  (params (Attacker :type "Character Object Reference") (Victim :type "Character Object Reference") (CinematicSetting :type "/Game/CounterAttackSystem/Blueprint/Struct/S_CinematicSettings Structure") (`Activate?` :type Boolean))
  (bind ((`CinematicCameraActor_69_2D6007514D208A2B20A31F8568C4F998` _cinematiccameraactor) (`SpringArmLength_62_A200BA99491289B205013DB12E6B63F1` _springarmlength) (`SpringArmRotation_63_91ACBE4548BC470F17D58C90DC39F560` _springarmrotation) (`SpringArmTargetOffset_65_DBB088D2488D7A0FD5A25CAA5B79BDB1` _springarmtargetoffset) (`UseCameraFadeSwitchTransition?_87_DECDAFF841D0DECFAA41569E1A7BF05B` _usecamerafadeswitchtransition_) (`CameraSwitchBlendSpeed_52_3ADDCAE647A2B145FD2CF8A4BC6B984C` _cameraswitchblendspeed) (`HoldtimeCounter_88_9E203B6C49E9817CD70B64B810EA6FB9` _holdtimecounter) (`DelaySwitchtoCameraDefault_72_8DEBDAE647891EC49B411BB6676ADC24` _delayswitchtocameradefault) (`CameraFocusTrackingTarget_89_C74AF44D49EDFBD5BE7CA4A25A8F5C62` _camerafocustrackingtarget) (`ManualFocusDistance_92_60C46F3D4C6BF1EFFB032889AAD3D4CE` _manualfocusdistance)) (break `/Game/CounterAttackSystem/Blueprint/Struct/S_CinematicSettings` CinematicSetting))
  (bind ((`UseCinematicCamera?_50_520533EA4FD000095C4B4381EFEA064C` _usecinematiccamera_) (`UseCameraFadeSwitchTransition?_87_DECDAFF841D0DECFAA41569E1A7BF05B` _usecamerafadeswitchtransition__2)) (break `/Game/CounterAttackSystem/Blueprint/Struct/S_CinematicSettings` CinematicSetting))
  ;[0 0.05001 0.09896] Cinematic Camera
  (if _usecinematiccamera_
    (`self.Multicast_InputSetting` Attacker) ; Disable Input Attacker
    (if (and (`KismetSystemLibrary.IsValid` Attacker) (`KismetSystemLibrary.IsValid` Victim))
      (if `Activate?`
        (bind _returnvalue (`|SpawnActorFromClass` _cinematiccameraactor (`Actor.GetTransform` Attacker) "AlwaysSpawn" "OverrideRootScale" Attacker null))
        (bind _ascs_cinematic_actor (cast `/Game/CounterAttackSystem/Blueprint/Camera/CAS_CinematicActor` _returnvalue))
        (bind _output_get (set `self.Counter_CameraActor` _ascs_cinematic_actor))
        (`/Engine/EditorBlueprintResources/StandardMacros.IsValid` (`Actor.GetComponentByClass` Attacker "/Script/Engine.SpringArmComponent")
          (:`Is Valid`
            (bind _cinecamera (`/Game/CounterAttackSystem/Blueprint/Camera/CAS_CinematicActor.Cinematic Camera Settings` _output_get Attacker Victim _springarmlength (`KismetMathLibrary.MakeRotator` (+ (.roll (`Pawn.GetControlRotation` Attacker)) (.roll _springarmrotation)) (+ (.pitch (`Pawn.GetControlRotation` Attacker)) (.pitch _springarmrotation)) (+ (.yaw (`Pawn.GetControlRotation` Attacker)) (.yaw _springarmrotation))) _springarmtargetoffset (`self.Draw Debug Camera Tracking`) _camerafocustrackingtarget _manualfocusdistance))
            (set `self.Counter_CineCamera` _cinecamera)
            (`self.Switch & Fade Camera` Attacker (`self.Counter_CineCamera`) _cameraswitchblendspeed _usecamerafadeswitchtransition__2) ; Switch camera Attacker
          ))
        (else
          (`KismetSystemLibrary.Delay` _delayswitchtocameradefault)
          (`self.Switch & Fade Camera` Attacker Attacker _cameraswitchblendspeed) ; Switch camera Attacker
          ;;[1 1 1] Set enable input after camera switch back to default
          (`KismetSystemLibrary.Delay` _cameraswitchblendspeed)
          (`self.Multicast_InputSetting` Attacker true) ; Enable Input Attacker
          (bind _counter_cameraactor (`self.Counter_CameraActor`)
            (:`then`
              (bind _counter_cinecamera (`self.Counter_CineCamera`)
                (:`then`
                  (`Actor.K2_DestroyActor` _counter_cameraactor)
                  (`Actor.K2_DestroyActor` _counter_cinecamera))
                (:`else`)))
            (:`else`)))))))

(event `Server_PlayMontage`
  (params (Character :type "Character Object Reference") (Montage :type "AnimMontage Object Reference") (PlayRate :type "Float (double-precision)"))
  ;[0 0.05001 0.09896] Animation Montage
  (`self.Multicast_PlayMontage` Character Montage PlayRate))

(event `Multicast_PlayMontage`
  (params (Character :type "Character Object Reference") (Montage :type "AnimMontage Object Reference") (PlayRate :type "Float (double-precision)"))
  ;[0 0.05001 0.09896] Animation Montage
  (`|PlayMontage` (`Character.Mesh` Character) Montage PlayRate
    (:`OnCompleted`
      _)
    (:`OnInterrupted`
      _))
  (`/Engine/EditorBlueprintResources/ActorComponentMacros.Switch Has Authority`
    (:`Authority`
      (`self.End Counter`))))

(event `MoveRotateAttackerToVictim`
  (params (Attacker :type "Character Object Reference") (Victim :type "Character Object Reference") (MatchingDistance :type "Float (double-precision)") (MatchingRotation :type "Float (double-precision)") (Direction :type "/Game/CounterAttackSystem/Blueprint/Enum/E_TriggerCounterDirection Enum" :default "NewEnumerator0"))
  (bind (_returnvalue_roll _returnvalue_pitch) (`KismetMathLibrary.BreakRotator` (`Actor.K2_GetActorRotation` Attacker)))
  ;[0 0.05001 0.09896] Move & Rotate Attacker to Victim
  (`self.Server_MoveComponentTo` (- (- (`Actor.K2_GetActorLocation` Victim) (* (`Actor.GetActorForwardVector` Victim) MatchingDistance)) (* (`Actor.GetActorRightVector` Victim) 0.0)) (`KismetMathLibrary.MakeRotator` _returnvalue_roll _returnvalue_pitch (+ (.yaw (`KismetMathLibrary.FindLookAtRotation` (`Actor.K2_GetActorLocation` Attacker) (`Actor.K2_GetActorLocation` Victim))) MatchingRotation)) Attacker)
  (`self.Server_Pawn_Collision_Response` "ECR_Ignore" (`self.OwnerAttacker`)))

(event `DeadRagdoll`
  (params (Delay :type "Float (double-precision)") (Character :type "Character Object Reference"))
  ;[0 0.05001 0.09896] Dead System
  (if (`self.UseDeadSystem`)
    (`KismetSystemLibrary.Delay` Delay)
    (`self.Server_DeadRagdoll` Character)
    (`Actor.SetLifeSpan` Character (`self.DeadLifespan`))
    (`self.OnOwnerDead_(Victim)`)))

(event `Server_MoveComponentTo`
  (params (TargetLocation :type "Vector Structure") (TargetRotation :type "Rotator Structure") (Attacker :type "Character Object Reference"))
  ;[0 0.05001 0.09896] Move & Rotate Attacker to Victim
  ;;[1 1 1] Network Move Component To
  (`self.Multicast_MoveComponentTo` TargetLocation TargetRotation Attacker))

(event `Server_DeadRagdoll`
  (params (Character :type "Character Object Reference"))
  ;[0 0.05001 0.09896] Dead System
  ;;[1 1 1] Ragdoll Death
  (`self.Multicast_DeadRagdoll` Character))

(event `Multicast_MoveComponentTo`
  (params (TargetLocation :type "Vector Structure") (TargetRotation :type "Rotator Structure") (Attacker :type "Character Object Reference"))
  ;[0 0.05001 0.09896] Move & Rotate Attacker to Victim
  ;;[1 1 1] Network Move Component To
  (`KismetSystemLibrary.MoveComponentTo` (`Character.CapsuleComponent` Attacker) TargetLocation TargetRotation false false 0.2 true))

(event `Multicast_DeadRagdoll`
  (params (Character :type "Character Object Reference"))
  (bind _mesh (`Character.Mesh` Character))
  ;[0 0.05001 0.09896] Dead System
  ;;[1 1 1] Ragdoll Death
  (`PrimitiveComponent.SetSimulatePhysics` _mesh true)
  (`PrimitiveComponent.SetCollisionProfileName` _mesh "Ragdoll" true)
  (`PrimitiveComponent.SetCollisionResponseToChannel` _mesh "ECC_Camera" "ECR_Ignore")
  (`PrimitiveComponent.SetCollisionEnabled` (`Character.CapsuleComponent` Character) "NoCollision")
  (set `self.IsOwnerDead` true))

(event `Switch & Fade Camera`
  (params (Character :type "Character Object Reference") (`New View Target` :type "Actor Object Reference") (BlendTime :type "Float (double-precision)") (`UseCameraFade?` :type Boolean))
  ;[0 0.05001 0.09896] Cinematic Camera
  ;;[1 1 1] Switch camera & give fade effect
  (bind _asplayer_controller (cast `PlayerController` (`Pawn.GetController` Character)))
  (if `UseCameraFade?`
    (`PlayerCameraManager.StartCameraFade` :`self` (`PlayerController.PlayerCameraManager` _asplayer_controller) :`FromAlpha` 1.3 :`Duration` 0.5))
  (`PlayerController.SetViewTargetWithBlend` _asplayer_controller `New View Target` BlendTime "VTBlend_Cubic" 0.0 false))

(event `Server_StartAttack`
  ;[0.09896 0.01421 0.08334] Simple AI random Attack to Player
  (if (not (`self.IsOwnerDead`))
    (bind _ascharacter (cast `Character` (`self.GetOwner`)))
    (`self.Server_PlayMontage` _ascharacter (select `int` (`KismetMathLibrary.RandomIntegerInRange` 0 2) :`0` "/Game/CounterAttackSystem/Animation/Attack/Attack_RightHand_Montage.Attack_RightHand_Montage" :`1` "/Game/CounterAttackSystem/Animation/Attack/Attack_LeftHand_Montage.Attack_LeftHand_Montage" :`2` "/Game/CounterAttackSystem/Animation/Attack/Attack_RightKick_Montage.Attack_RightKick_Montage" :!type "AnimMontage Object Reference") 1.0)))

(event `Server_Pawn_Collision_Response`
  (params (Response :type "ECollisionResponse Enum" :default "ECR_Ignore") (Character :type "Character Object Reference"))
  ;[0 0.05001 0.09896] Pawn Collision Response
  (`self.Multicast_Pawn_Collision_Response` Response Character))

(event `Multicast_InputSetting`
  (params (Character :type "Character Object Reference") (Enable :type Boolean))
  ;[0 0.05001 0.09896] Input Setting
  (`/Engine/EditorBlueprintResources/StandardMacros.IsValid` Character
    (:`Is Valid`
      (bind _asplayer_controller (cast `PlayerController` (`Pawn.GetController` Character)))
      (if Enable
        (`Actor.EnableInput` Character _asplayer_controller)
        (else
          (`Actor.DisableInput` Character _asplayer_controller))))))

(event `Multicast_Pawn_Collision_Response`
  (params (Response :type "ECollisionResponse Enum" :default "ECR_Ignore") (Character :type "Character Object Reference"))
  ;[0 0.05001 0.09896] Pawn Collision Response
  (`/Engine/EditorBlueprintResources/StandardMacros.IsValid` Character
    (:`Is Valid`
      (`PrimitiveComponent.SetCollisionResponseToChannel` (`Character.CapsuleComponent` Character) "ECC_Pawn" Response))))

(event `OpenClose_Counter`
  (params (Open :type Boolean) (CounterType :type "/Game/CounterAttackSystem/Blueprint/Enum/E_CounterType Enum" :default "NewEnumerator0") (Initiator :type "Actor Object Reference"))
  ;[0 0.05001 0.09896] Open Close Counter
  (bind _output_get (set `self.CanCounter?` Open))
  (if _output_get
    (set `self.SendingCounterType` CounterType)
    (`self.OnOpenCounter` Initiator)
    (else
      (if (`self.InCounter`)
        (`KismetSystemLibrary.Delay` 0.5) ; If in counter give a bit delay before close counter
      )
      (`self.OnCloseCounter` Initiator))))

(event `Server_PlaySound`
  (params (Sound :type "SoundCue Object Reference") (Location :type "Vector Structure"))
  ;[0 0.05001 0.09896] Play Sound
  (`self.Multicast_PlaySound` Sound Location))

(event `Multicast_PlaySound`
  (params (Sound :type "SoundCue Object Reference") (Location :type "Vector Structure"))
  ;[0 0.05001 0.09896] Play Sound
  (`GameplayStatics.PlaySoundAtLocation` Sound Location (struct) 1.0 1.0 0.0 null null null null))

(event `Server_PlayCameraShake`
  (params (CameraShake :type "CameraShakeBase Class Reference") (Location :type "Vector Structure"))
  ;[0 0.05001 0.09896] Play Camera Shake
  (`self.Client_PlayCameraShake` CameraShake Location))

(event `Client_PlayCameraShake`
  (params (CameraShake :type "CameraShakeBase Class Reference") (Location :type "Vector Structure"))
  ;[0 0.05001 0.09896] Play Camera Shake
  (`GameplayStatics.PlayWorldCameraShake` CameraShake Location 0.0 1000.0))

(fn `FindCounterDirection`
  (params (OwnerAttacker :type "Actor Object Reference") (Direction :type "Vector Structure"))
  (returns (CounterDirection :type "/Game/CounterAttackSystem/Blueprint/Enum/E_TriggerCounterDirection Enum"))
  (locals (L_DotProduct :type "Float (double-precision)"))
  ;[1 1 1] Find counter direction from victim perspective
  (`/Engine/EditorBlueprintResources/StandardMacros.IsValid` OwnerAttacker
    (:`Is Valid`
      (set `local.L_DotProduct` (`KismetMathLibrary.Dot_VectorVector` (`KismetMathLibrary.Normal` (`KismetMathLibrary.MakeVector` (.x (`Actor.GetActorForwardVector` OwnerAttacker)) (.y (`Actor.GetActorForwardVector` OwnerAttacker)))) (`KismetMathLibrary.Normal` (`KismetMathLibrary.MakeVector` (.x Direction) (.y Direction)))))
      (`|ExecutionSequence`
        (:`then_0`
          (if (>= (`local.L_DotProduct`) 0.35)
            (return "NewEnumerator1")))
        (:`then_1`
          (if (<= (`local.L_DotProduct`) -0.35)
            (return "NewEnumerator0")))
        (:`then_2`
          (bind _output_get (set `local.L_DotProduct` (`KismetMathLibrary.Dot_VectorVector` (`KismetMathLibrary.Normal` (`KismetMathLibrary.MakeVector` (.x (`Actor.GetActorRightVector` OwnerAttacker)) (.y (`Actor.GetActorRightVector` OwnerAttacker)))) (`KismetMathLibrary.Normal` (`KismetMathLibrary.MakeVector` (.x Direction) (.y Direction))))))
          (if (>= _output_get 0.0)
            (return "NewEnumerator2")
            (else
              (return "NewEnumerator3"))))))
    (:`Is Not Valid`
      (return "NewEnumerator0"))))

(fn `Get Counter Settings`
  (params (`Counter Data` :type "/Game/CounterAttackSystem/Blueprint/Struct/S_CounterData Structure") (CounterType :type "/Game/CounterAttackSystem/Blueprint/Enum/E_CounterType Enum" :default "NewEnumerator4"))
  (returns (`Counter Settings Direction` :type "/Game/CounterAttackSystem/Blueprint/Struct/S_CounterSetting Structure") (CounterDirection :type "/Game/CounterAttackSystem/Blueprint/Enum/E_TriggerCounterDirection Enum") (`Success?` :type Boolean))
  (locals (L_CounterType :type "/Game/CounterAttackSystem/Blueprint/Enum/E_CounterType Enum" :default "NewEnumerator4") (L_CounterDirection :type "/Game/CounterAttackSystem/Blueprint/Enum/E_TriggerCounterDirection Enum" :default "NewEnumerator0"))
  (bind (_frontcounter _backcounter _leftcounter _rightcounter) (break `/Game/CounterAttackSystem/Blueprint/Struct/S_CounterData` `Counter Data`))
  (bind _ownerattacker (`self.OwnerAttacker`))
  (bind _countertype (break `/Game/CounterAttackSystem/Blueprint/Struct/S_CounterType` (select `/Game/CounterAttackSystem/Blueprint/Enum/E_TriggerCounterDirection` (`local.L_CounterDirection`) :`NewEnumerator0` _frontcounter :`NewEnumerator1` _frontcounter :`NewEnumerator2` _frontcounter :`NewEnumerator3` _frontcounter)))
  (bind (_value _returnvalue) (`BlueprintMapLibrary.Map_Find` _countertype (`local.L_CounterType`)))
  (bind (_value_2 _returnvalue_2) (`BlueprintMapLibrary.Map_Find` (`.CounterType_66_578CC4034598A8CDCE09D9820367B566` (break `/Game/CounterAttackSystem/Blueprint/Struct/S_CounterType` (select `/Game/CounterAttackSystem/Blueprint/Enum/E_TriggerCounterDirection` (`local.L_CounterDirection`) :`NewEnumerator0` _frontcounter :`NewEnumerator1` _backcounter :`NewEnumerator2` _leftcounter :`NewEnumerator3` _rightcounter))) (`local.L_CounterType`)))
  (bind (_countersettings _playrandommontage) (break `/Game/CounterAttackSystem/Blueprint/Struct/S_CounterSettingArray` _value_2))
  (bind (_countersettings_2 _playrandommontage_2) (break `/Game/CounterAttackSystem/Blueprint/Struct/S_CounterSettingArray` (select `bool` _returnvalue :`false` (`BlueprintMapLibrary.Map_Find` _countertype "NewEnumerator0") :`true` _value)))
  (bind _output (`|GetArrayItem` _countersettings (select `bool` _playrandommontage :`true` (`KismetMathLibrary.RandomInteger` (`KismetArrayLibrary.Array_Length` _countersettings)))))
  (bind _returnvalue_3 (select `bool` _playrandommontage_2 :`true` (`KismetMathLibrary.RandomInteger` (`KismetArrayLibrary.Array_Length` _countersettings_2))))
  (bind _output_2 (`|GetArrayItem` _countersettings_2 _returnvalue_3))
  (bind ((`AttackerMontage_11_9E203B6C49E9817CD70B64B810EA6FB9` _attackermontage) (`VictimMontage_12_E79B1A724393874BA00E2A951C02C4D2` _victimmontage)) (break `/Game/CounterAttackSystem/Blueprint/Struct/S_CounterMontageSetting` (`.MontageSettings_49_9E203B6C49E9817CD70B64B810EA6FB9` (break `/Game/CounterAttackSystem/Blueprint/Struct/S_CounterSetting` _output))))
  (bind ((`AttackerMontage_11_9E203B6C49E9817CD70B64B810EA6FB9` _attackermontage_2) (`VictimMontage_12_E79B1A724393874BA00E2A951C02C4D2` _victimmontage_2)) (break `/Game/CounterAttackSystem/Blueprint/Struct/S_CounterMontageSetting` (`.MontageSettings_49_9E203B6C49E9817CD70B64B810EA6FB9` (break `/Game/CounterAttackSystem/Blueprint/Struct/S_CounterSetting` _output_2))))
  ;[1 1 1] Find the correct montage, distance & rotation base on direction. If there is direction Counter doesn't have montage then always start Counter Front.
  (set `local.L_CounterType` CounterType)
  (set `local.L_CounterDirection` (`self.FindCounterDirection` _ownerattacker (`KismetMathLibrary.GetDirectionUnitVector` (`Actor.K2_GetActorLocation` (`self.CounterVictim`)) (`Actor.K2_GetActorLocation` _ownerattacker))))
  (if _returnvalue_2
    (if (and (`KismetSystemLibrary.IsValid` _attackermontage) (`KismetSystemLibrary.IsValid` _victimmontage))
      (return _output (`local.L_CounterDirection`) true)
      (else
        (if (and (`KismetSystemLibrary.IsValid` _attackermontage_2) (`KismetSystemLibrary.IsValid` _victimmontage_2)) :!label _label
          _
          (else
            (return (struct) "NewEnumerator0" false)))))
    (elif (`KismetArrayLibrary.Array_IsValidIndex` _countersettings_2 _returnvalue_3)
      (goto _label)
      (else
        (return (struct) "NewEnumerator0" false))))
  (return _output_2 "NewEnumerator0" true))